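; BP_Shop is a shop actor that the player opens on demand while standing in its trigger volume.
; Entering PopUpTrigger shows a W_PopUp prompt and enables input; leaving it removes all widgets.
; Pressing OpenShop while overlapping swaps the prompt for W_ShopUI, blends the camera to the shop actor and switches to UI-only input with a visible cursor.
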(event `self.PopUp Trigger.OnComponentBeginOverlap`
  (params (OverlappedComponent :type "PrimitiveComponent Object Reference") (OtherActor :type "Actor Object Reference") (OtherComp :type "PrimitiveComponent Object Reference") (OtherBodyIndex :type Integer) (bFromSweep :type Boolean) (SweepResult :type "HitResult Structure (by ref)"))
  (bind _returnvalue (`|CreateWidget` "/Game/Widgets/W_PopUp.W_PopUp_C"))
  (bind _output_get (set `self.PopUp` _returnvalue))
  (`UserWidget.AddToViewport` _output_get 0)
  (`self.EnableInput` null)
  (set `self.Overlapping` true))

(event `self.PopUp Trigger.OnComponentEndOverlap`
  (params (OverlappedComponent :type "PrimitiveComponent Object Reference") (OtherActor :type "Actor Object Reference") (OtherComp :type "PrimitiveComponent Object Reference") (OtherBodyIndex :type Integer))
  (`WidgetLayoutLibrary.RemoveAllWidgets`)
  (set `self.Overlapping` false))

(event `InputAction|OpenShop`
  (params (Key :type "Key Structure"))
  (bind _returnvalue (`GameplayStatics.GetPlayerController` 0))
  (:`Pressed`
    (if (`self.Overlapping`)
      (`Widget.RemoveFromParent` (`self.PopUp`))
      (`PlayerController.SetViewTargetWithBlend` (`GameplayStatics.GetPlayerController` 0) self 1.0 "VTBlend_Linear" 0.0 false)
      (bind _returnvalue_2 (`|CreateWidget` "/Game/Widgets/W_ShopUI.W_ShopUI_C"))
      (bind _output_get (set `self.ShopUI` _returnvalue_2))
      (`UserWidget.AddToViewport` _output_get 0)
      (`WidgetBlueprintLibrary.SetInputMode_UIOnlyEx` _returnvalue _output_get)
      (set `PlayerController.bShowMouseCursor` true _returnvalue))))

(fn `UserConstructionScript`)